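; Glass staircase actor that destroys itself when anything stops overlapping the trigger box at its far end.
; The Construction Script repeats a static mesh every 200 units along the StairEnd vector, yawed to face that direction.
; It then adds a scaled box just above the last step and stores it as BoxCollision, whose end-overlap event destroys the whole actor without filtering what left.
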(event OnComponentEndOverlap(BoxCollision)
  (params (OverlappedComponent :type Primitive%20Component%20Object%20Reference) (OtherActor :type Actor%20Object%20Reference) (OtherComp :type Primitive%20Component%20Object%20Reference) (OtherBodyIndex :type Integer))
  (Actor|DestroyActor))

(event EventBeginPlay)

(event Collision|EventActorBeginOverlap
  (params (OtherActor :type Actor%20Object%20Reference)))

(event EventTick
  (params (DeltaSeconds :type Float%20%28single-precision%29)))

(fn ConstructionScript
  (bind _stairend (Variables|Default|GetStairEnd))
  (bind _returnvalue (Math|Vector|VectorLength _stairend))
  (bind _returnvalue_2 (/ _returnvalue 2e+02))
  (bind _returnvalue_3 (Math|Float|Truncate _returnvalue_2))
  (Variables|Default|SetStairDirection (Math|Vector|Normalize _stairend))
  (for _index (range 0 _returnvalue_3)
    (AddComponent|AddStaticMeshComponent false (Math|Transform|MakeTransform (* _index 200 (Variables|Default|GetStairDirection)) (Math|Rotator|MakeRotator 0.0 0.0 (.yaw (Math|Conversions|RotationFromXVector (Variables|Default|GetStairDirection)))) "1.000000,1.000000,1.000000")))
  (bind _returnvalue_4 (AddComponent|AddBoxComponent false (Math|Transform|MakeTransform (+ (* _returnvalue_3 200 (Variables|Default|GetStairDirection)) "0.000000,0.000000,30.000000") (Math|Rotator|MakeRotator 0.0 0.0 (.yaw (Math|Conversions|RotationFromXVector (Variables|Default|GetStairDirection)))) "3.000000,3.000000,0.500000")))
  (Variables|Default|SetBoxCollision _returnvalue_4))