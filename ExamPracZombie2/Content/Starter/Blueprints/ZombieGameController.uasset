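; Player controller that flies an aircraft pawn and lets the player eject from it as a granny character.
; Enhanced Input actions drive yaw, pitch and forward/right movement for the aircraft, with a separate look action for the granny.
; Space spawns a granny at the airplane's DropPoint, possesses it and swaps the aircraft mapping context for the granny one.
; The abandoned airplane then simulates physics and is flagged as ejected.
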(event Input|EnhancedActionEvents|EnhancedInputActionIA_RotateGranny
  (params (ActionValue :type Vector%202D%20Structure) (ElapsedSeconds :type Float%20%28double-precision%29) (TriggeredSeconds :type Float%20%28double-precision%29) (InputAction :type Input%20Action%20Object%20Reference :default "/Game/Starter/Assets/Inputs/IA_RotateGranny.IA_RotateGranny"))
  (Class|PlayerController|AddYawInput (.x ActionValue))
  (Class|PlayerController|AddPitchInput (.y ActionValue)))

(event Input|EnhancedActionEvents|EnhancedInputActionIA_RotateAircraft
  (params (ActionValue :type Vector%202D%20Structure) (ElapsedSeconds :type Float%20%28double-precision%29) (TriggeredSeconds :type Float%20%28double-precision%29) (InputAction :type Input%20Action%20Object%20Reference :default "/Game/Starter/Assets/Inputs/IA_RotateAircraft.IA_RotateAircraft"))
  (Class|PlayerController|AddYawInput (.x ActionValue))
  (Class|PlayerController|AddPitchInput (.y ActionValue)))

(event Input|EnhancedActionEvents|EnhancedInputActionIA_MoveAircraft
  (params (ActionValue :type Vector%202D%20Structure) (ElapsedSeconds :type Float%20%28double-precision%29) (TriggeredSeconds :type Float%20%28double-precision%29) (InputAction :type Input%20Action%20Object%20Reference :default "/Game/Starter/Assets/Inputs/IA_MoveAircraft.IA_MoveAircraft"))
  (bind _returnvalue (Pawn|GetControlledPawn))
  (Pawn|Input|AddMovementInput _returnvalue (Transformation|GetActorForwardVector _returnvalue) (.x ActionValue) false)
  (Pawn|Input|AddMovementInput _returnvalue (Transformation|GetActorRightVector _returnvalue) (.y ActionValue) false))

(event EventBeginPlay
  (Input|AddMappingContext (PlayerController|LocalPlayerSubsystems|GetEnhancedInputLocalPlayerSubsystem) "/Game/Starter/Assets/Inputs/IMC_AircraftControl.IMC_AircraftControl" 0 "(bIgnoreAllPressedKeysUntilRelease=True,bForceImmediately=False,bNotifyUserSettings=False)"))

(event EventTick
  (params (DeltaSeconds :type Float%20%28single-precision%29)))

(event Input|KeyboardEvents|SpaceBar
  (params (Key :type Key%20Structure :default "None"))
  (bind _returnvalue (PlayerController|LocalPlayerSubsystems|GetEnhancedInputLocalPlayerSubsystem))
  (:Pressed
    (bind _asbp_airplane (Utilities|Casting|CastToBP_Airplane (Pawn|GetControlledPawn)))
    (bind _returnvalue_2 (Game|SpawnActorfromClass "/Game/Starter/Blueprints/Granny.Granny_C" (Transformation|GetWorldTransform (Variables|/Game/Starter/Blueprints/BP_Airplane.BP_Airplane_C|GetDropPoint _asbp_airplane)) "Undefined" "MultiplyWithRoot" 0 0))
    (Pawn|Possess _returnvalue_2)
    (Input|RemoveMappingContext _returnvalue "/Game/Starter/Assets/Inputs/IMC_AircraftControl.IMC_AircraftControl" "(bIgnoreAllPressedKeysUntilRelease=True,bForceImmediately=False,bNotifyUserSettings=False)")
    (Input|AddMappingContext _returnvalue "/Game/Starter/Assets/Inputs/IMC_GrannyControl.IMC_GrannyControl" 0 "(bIgnoreAllPressedKeysUntilRelease=True,bForceImmediately=False,bNotifyUserSettings=False)")
    (Physics|SetSimulatePhysics (Variables|/Game/Starter/Blueprints/BP_Airplane.BP_Airplane_C|GetStaticMesh _asbp_airplane) true)
    (Variables|/Game/Starter/Blueprints/BP_Airplane.BP_Airplane_C|SetEject? _asbp_airplane true)))

(fn ConstructionScript)