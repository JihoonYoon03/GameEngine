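; Granny player character with camera-relative movement, jumping, and a rifle that becomes aimable once GetWeapon arms her.
; Right mouse switches to an over-the-shoulder aim with a debug trace; left mouse plays the fire montage, line-tracing from the muzzle while aiming to spawn explosions and apply damage.
; After an eject, she must press jump within range of the ground or die on touchdown.
; Any damage also kills her and disables input.
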(event Custom|GetWeapon
  (Variables|Default|SetArmed? true)
  (Rendering|SetVisibility (Variables|Default|GetSpotLight) true false)
  (Audio|PlaySound2D "/Engine/VREditor/Sounds/UI/Camera_Shutter.Camera_Shutter" 1.0 1.0 0.0 0 0))

(event Input|EnhancedActionEvents|EnhancedInputActionIA_MoveGranny
  (params (ActionValue :type Vector%202D%20Structure) (ElapsedSeconds :type Float%20%28double-precision%29) (TriggeredSeconds :type Float%20%28double-precision%29) (InputAction :type Input%20Action%20Object%20Reference :default "/Game/Starter/Assets/Inputs/IA_MoveGranny.IA_MoveGranny"))
  (bind _returnvalue (Pawn|GetControlRotation :!class /Script/Engine.Pawn))
  ;[0.15 0.15 0.15 0.5] RPG Style
  (Pawn|Input|AddMovementInput (Math|Vector|GetForwardVector (Math|Rotator|MakeRotator 0.0 0.0 (.yaw _returnvalue))) (.x ActionValue) false)
  (Pawn|Input|AddMovementInput (Math|Vector|GetRightVector (Math|Rotator|MakeRotator 0.0 0.0 (.yaw _returnvalue))) (.y ActionValue) false))

(event Input|EnhancedActionEvents|EnhancedInputActionIA_JumpGranny
  (params (ActionValue :type Boolean) (ElapsedSeconds :type Float%20%28double-precision%29) (TriggeredSeconds :type Float%20%28double-precision%29) (InputAction :type Input%20Action%20Object%20Reference :default "/Game/Starter/Assets/Inputs/IA_JumpGranny.IA_JumpGranny"))
  (bind _returnvalue (Transformation|GetActorLocation))
  (:Started
    (if (Variables|Default|GetAfterEject?)
      (bind (_outhit _returnvalue_2) (Collision|LineTraceByChannel _returnvalue (- _returnvalue "0.000000,0.000000,2000.000000") "TraceTypeQuery1" false 0 "ForOneFrame"))
      (if _returnvalue_2
        (if (Math|Float|InRange(Float) (.distance _outhit) 0.0 1.5e+03)
          (Variables|Default|SetLanded true)))
      (else
        (Character|Jump)))))

(event EventBeginPlay)

(event Collision|EventActorBeginOverlap
  (params (OtherActor :type Actor%20Object%20Reference)))

(event EventTick
  (params (DeltaSeconds :type Float%20%28single-precision%29))
  (bind _muzzle (Variables|Default|GetMuzzle))
  (bind _returnvalue (Transformation|GetWorldLocation _muzzle))
  (Variables|Default|SetSpeed (Math|Vector|VectorLengthXY (Transformation|GetVelocity)))
  (if (Variables|Default|GetAfterEject?)
    (if (AI|Components|NavMovement|IsMovingonGround (Variables|Character|GetCharacterMovement))
      (if (Variables|Default|GetLanded)
        (Variables|Default|SetAfterEject? false)
        (else
          (Input|DisableInput 0)
          (Variables|Default|SetDead true))))
    (elif (Variables|Default|GetAiming?)
      (Collision|LineTraceByChannel _returnvalue (+ _returnvalue (* (Math|Vector|GetForwardVector _muzzle) 1e+04)) "TraceTypeQuery2" false 0 "ForOneFrame"))))

(event Game|Damage|EventAnyDamage
  (params (Damage :type Float%20%28single-precision%29) (DamageType :type Damage%20Type%20Object%20Reference) (InstigatedBy :type Controller%20Object%20Reference) (DamageCauser :type Actor%20Object%20Reference))
  (Input|DisableInput 0)
  (Variables|Default|SetDead true))

(event Input|MouseEvents|RightMouseButton
  (params (Key :type Key%20Structure :default "None"))
  (bind _armed_ (Variables|Default|GetArmed?))
  (bind _charactermovement (Variables|Character|GetCharacterMovement))
  (bind _springarm (Variables|Default|GetSpringArm))
  (bind _camera (Variables|Default|GetCamera))
  (:Pressed
    (if _armed_
      (Variables|Default|SetAiming? true)
      (Variables|/Script/Engine.CharacterMovementComponent|SetbOrientRotationToMovement _charactermovement false)
      (Variables|Default|SetbUseControllerRotationYaw true)
      (Variables|/Script/Engine.SpringArmComponent|SetTargetArmLength _springarm 1.5e+02)
      (Transformation|SetRelativeLocation _camera "0.000000,80.000000,50.000000" false false)
      (Animation|Montage|PlayMontage (Variables|Character|GetMesh) "/Game/Starter/Assets/Granny/Animations/GrannyRifleMontage.GrannyRifleMontage" 1.0 0.0 "Look")))
  (:Released
    (if _armed_
      (Variables|Default|SetAiming? false)
      (Variables|/Script/Engine.CharacterMovementComponent|SetbOrientRotationToMovement _charactermovement true)
      (Variables|Default|SetbUseControllerRotationYaw false)
      (Variables|/Script/Engine.SpringArmComponent|SetTargetArmLength _springarm 3e+02)
      (Transformation|SetRelativeLocation _camera "0.000000,0.000000,0.000000" false false)
      (Animation|StopAnimMontage "/Game/Starter/Assets/Granny/Animations/GrannyRifleMontage.GrannyRifleMontage"))))

(event Input|MouseEvents|LeftMouseButton
  (params (Key :type Key%20Structure :default "None"))
  (:Pressed
    (bind (_outhit _hit_) (CallFunction|Shoot))
    (Animation|Montage|PlayMontage (Variables|Character|GetMesh) "/Game/Starter/Assets/Granny/Animations/GrannyRifleMontage.GrannyRifleMontage" 1.0 0.0 "Fire"
      (:then
        (Audio|PlaySoundatLocation "/Game/Starter/Assets/Rifle/Audio/FirstPersonTemplateWeaponFire02.FirstPersonTemplateWeaponFire02" (Transformation|GetActorLocation) "0, 0, 0" 1.0 1.0 0.0 0 0 0 0)
        (if _hit_
          (Effects|SpawnEmitteratLocation "/Game/StarterContent/Particles/P_Explosion.P_Explosion" (.location _outhit) "0, 0, 0" "0.300000,0.300000,0.300000")
          (Game|Damage|ApplyDamage (.hitactor _outhit) 1e+02 0 0 "/Script/Engine.DamageType"))))))

(fn ConstructionScript)

(fn Shoot
  (bind _muzzle (Variables|Default|GetMuzzle))
  (bind _returnvalue (Transformation|GetWorldLocation _muzzle))
  (if (Variables|Default|GetAiming?)
    (bind (_outhit _returnvalue_2) (Collision|LineTraceByChannel _returnvalue (+ _returnvalue (* (Math|Vector|GetForwardVector _muzzle) 1e+04)) "TraceTypeQuery2" false 0 "ForOneFrame"))
    (return _outhit _returnvalue_2)))