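; Zombie enemy that chases the Granny player pawn and deals damage to whatever its capsule hits.
; Each Tick while alive, Chase picks a fast or slow walk speed by distance and yaw toward the player drives movement input, stopping beyond range.
; Damage lowers Health, and at zero it sets Dead and disables capsule collision.
; A separate Dissolve event sets a lifespan but also destroys the actor immediately.
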(event OnComponentHit(CapsuleComponent)
  (params (HitComponent :type Primitive%20Component%20Object%20Reference) (OtherActor :type Actor%20Object%20Reference) (OtherComp :type Primitive%20Component%20Object%20Reference) (NormalImpulse :type Vector :default "0, 0, 0") (Hit :type Hit%20Result%20Structure%20%28by%20ref%29))
  (Game|Damage|ApplyDamage OtherActor 1.0 0 0 "/Script/Engine.DamageType"))

(event Custom|Dissolve
  (Actor|SetLifeSpan 3.0)
  (Actor|DestroyActor))

(event EventBeginPlay)

(event Collision|EventActorBeginOverlap
  (params (OtherActor :type Actor%20Object%20Reference)))

(event Game|Damage|EventAnyDamage
  (params (Damage :type Float%20%28single-precision%29) (DamageType :type Damage%20Type%20Object%20Reference) (InstigatedBy :type Controller%20Object%20Reference) (DamageCauser :type Actor%20Object%20Reference))
  (bind _output_get (Variables|Default|SetHealth (- (Variables|Default|GetHealth) Damage)))
  (if (<= _output_get 0.0)
    (Variables|Default|SetDead true)
    (Collision|SetCollisionEnabled (Variables|Collision|GetCapsuleComponent) "NoCollision")))

(event EventTick
  (params (DeltaSeconds :type Float%20%28single-precision%29))
  (if (not (Variables|Default|GetDead))
    (Variables|Default|SetSpeed (Math|Vector|VectorLengthXY (Transformation|GetVelocity)))
    (bind _found (CallFunction|Chase))
    (if _found
      (Pawn|Input|AddMovementInput (Math|Vector|GetForwardVector (Variables|Default|GetToPlayer)) 1.0 false))))

(fn ConstructionScript)

(fn Chase
  (bind _returnvalue (Game|Player|GetPlayerPawn 0))
  (bind _charactermovement (Variables|Character|GetCharacterMovement))
  (bind _returnvalue_2 (Transformation|GetDistanceTo _returnvalue))
  (Utilities|Casting|CastToGranny _returnvalue
    (:then
      (Variables|Default|SetToPlayer (Math|Rotator|MakeRotator 0.0 0.0 (.yaw (Math|Rotator|FindLookatRotation (Transformation|GetActorLocation) (Transformation|GetActorLocation _returnvalue)))))
      (if (Math|Float|InRange(Float) _returnvalue_2 0.0 1e+03)
        (Variables|/Script/Engine.CharacterMovementComponent|SetMaxWalkSpeed _charactermovement 257.0)
        (return true)
        (elif (Math|Float|InRange(Float) _returnvalue_2 1e+03 2.5e+03)
          (Variables|/Script/Engine.CharacterMovementComponent|SetMaxWalkSpeed _charactermovement 4e+01)
          (return true)
          (else
            _))))
    (:CastFailed
      _))
  (return false))