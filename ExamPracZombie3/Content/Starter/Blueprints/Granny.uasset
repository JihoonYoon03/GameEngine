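; Granny is a player character Blueprint with walk, sprint, jump, rifle combat and a survivable ejection fall.
; GetWeapon reveals the rifle and spotlight, enabling right-click aiming with a shoulder camera and montage; left-click fires a muzzle line trace for damage and explosion effects.
; While ejected, jump must be pressed near the ground (checked by a downward trace), or touchdown kills her.
; Any damage also sets Dead and disables input.
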(event Custom|GetWeapon
  (Variables|Default|SetArmed? true)
  (Rendering|SetVisibility (Variables|Default|GetRifle) true false))

(event Input|EnhancedActionEvents|EnhancedInputActionIA_MoveGranny
  (params (ActionValue :type Vector%202D%20Structure) (ElapsedSeconds :type Float%20%28double-precision%29) (TriggeredSeconds :type Float%20%28double-precision%29) (InputAction :type Input%20Action%20Object%20Reference :default "/Game/Starter/Assets/Inputs/IA_MoveGranny.IA_MoveGranny"))
  (bind _returnvalue (Pawn|GetControlRotation :!class /Script/Engine.Pawn))
  ;[0.15 0.15 0.15 0.5] RPG Style
  (Pawn|Input|AddMovementInput (Math|Vector|GetForwardVector (Math|Rotator|MakeRotator 0.0 0.0 (.yaw _returnvalue))) (.x ActionValue) false)
  (Pawn|Input|AddMovementInput (Math|Vector|GetRightVector (Math|Rotator|MakeRotator 0.0 0.0 (.yaw _returnvalue))) (.y ActionValue) false))

(event Input|EnhancedActionEvents|EnhancedInputActionIA_JumpGranny
  (params (ActionValue :type Boolean) (ElapsedSeconds :type Float%20%28double-precision%29) (TriggeredSeconds :type Float%20%28double-precision%29) (InputAction :type Input%20Action%20Object%20Reference :default "/Game/Starter/Assets/Inputs/IA_JumpGranny.IA_JumpGranny"))
  (bind _returnvalue (Transformation|GetActorLocation))
  (:Started
    (if (Variables|Default|GetEjectedNow?)
      (bind _outhit (Collision|LineTraceByChannel _returnvalue (- _returnvalue "0.000000,0.000000,2000.000000") "TraceTypeQuery1" false 0 "ForOneFrame"))
      (if (< (.distance _outhit) 1.2e+03)
        (Variables|Default|SetLanded true))
      (else
        (Character|Jump)))))

(event Input|EnhancedActionEvents|EnhancedInputActionIA_MoveGranny
  (params (ActionValue :type Vector%202D%20Structure) (ElapsedSeconds :type Float%20%28double-precision%29) (TriggeredSeconds :type Float%20%28double-precision%29) (InputAction :type Input%20Action%20Object%20Reference :default "/Game/Starter/Assets/Inputs/IA_MoveGranny.IA_MoveGranny"))
  (bind _returnvalue (Pawn|GetControlRotation :!class /Script/Engine.Pawn))
  (Pawn|Input|AddMovementInput (Math|Vector|GetForwardVector _returnvalue) (.x ActionValue) false)
  (Pawn|Input|AddMovementInput (Math|Vector|GetRightVector _returnvalue) (.y ActionValue) false))

(event EventBeginPlay)

(event Collision|EventActorBeginOverlap
  (params (OtherActor :type Actor%20Object%20Reference)))

(event EventTick
  (params (DeltaSeconds :type Float%20%28single-precision%29))
  (Variables|Default|SetSpeed (Math|Vector|VectorLengthXY (Transformation|GetVelocity)))
  (if (Variables|Default|GetEjectedNow?)
    (if (AI|Components|NavMovement|IsMovingonGround (Variables|Character|GetCharacterMovement))
      (if (Variables|Default|GetLanded)
        (Variables|Default|SetEjectedNow? false)
        (else
          (Variables|Default|SetDead true)
          (Input|DisableInput 0))))
    (elif (Variables|Default|GetAiming?)
      (CallFunction|ShootRay))))

(event Game|Damage|EventAnyDamage
  (params (Damage :type Float%20%28single-precision%29) (DamageType :type Damage%20Type%20Object%20Reference) (InstigatedBy :type Controller%20Object%20Reference) (DamageCauser :type Actor%20Object%20Reference))
  (Input|DisableInput 0)
  (Variables|Default|SetDead true))

(event Input|MouseEvents|RightMouseButton
  (params (Key :type Key%20Structure :default "None"))
  (bind _springarm (Variables|Default|GetSpringArm))
  (bind _armed_ (Variables|Default|GetArmed?))
  (bind _camera (Variables|Default|GetCamera))
  (bind _charactermovement (Variables|Character|GetCharacterMovement))
  (:Pressed
    (if _armed_
      (Variables|Default|SetAiming? true)
      (Variables|/Script/Engine.SpringArmComponent|SetTargetArmLength _springarm 1.5e+02)
      (Transformation|SetRelativeLocation _camera "0.000000,80.000000,50.000000" false false)
      (Variables|Default|SetbUseControllerRotationYaw true)
      (Variables|/Script/Engine.CharacterMovementComponent|SetbOrientRotationToMovement _charactermovement false)
      (Animation|Montage|PlayMontage (Variables|Character|GetMesh) "/Game/Starter/Assets/Granny/Animations/ShootingMontage.ShootingMontage" 1.0 0.0 "Aim")))
  (:Released
    (if _armed_
      (Variables|Default|SetAiming? false)
      (Variables|/Script/Engine.SpringArmComponent|SetTargetArmLength _springarm 3e+02)
      (Transformation|SetRelativeLocation _camera "0.000000,0.000000,0.000000" false false)
      (Variables|Default|SetbUseControllerRotationYaw false)
      (Variables|/Script/Engine.CharacterMovementComponent|SetbOrientRotationToMovement _charactermovement true)
      (Animation|StopAnimMontage "/Game/Starter/Assets/Granny/Animations/ShootingMontage.ShootingMontage"))))

(event Input|MouseEvents|LeftMouseButton
  (params (Key :type Key%20Structure :default "None"))
  (:Pressed
    (if (Variables|Default|GetAiming?)
      (Animation|Montage|PlayMontage (Variables|Character|GetMesh) "/Game/Starter/Assets/Granny/Animations/ShootingMontage.ShootingMontage" 1.0 0.0 "Fire"
        (:then
          (Audio|PlaySoundatLocation "/Game/Starter/Assets/Rifle/Audio/FirstPersonTemplateWeaponFire02.FirstPersonTemplateWeaponFire02" (Transformation|GetWorldLocation (Variables|Default|GetMuzzle)) "0, 0, 0" 1.0 1.0 0.0 0 0 0 0)
          (bind (_hitresult _hit) (CallFunction|ShootRay))
          (if _hit
            (Effects|SpawnEmitteratLocation "/Game/StarterContent/Particles/P_Explosion.P_Explosion" (.location _hitresult) "0, 0, 0" "0.300000,0.300000,0.300000")
            (Game|Damage|ApplyDamage (.hitactor _hitresult) 1e+02 0 0 "/Script/Engine.DamageType")))))))

(event Input|KeyboardEvents|LeftShift
  (params (Key :type Key%20Structure :default "None"))
  (bind _charactermovement (Variables|Character|GetCharacterMovement))
  (:Pressed
    (Variables|/Script/Engine.CharacterMovementComponent|SetMaxWalkSpeed _charactermovement 852.0))
  (:Released
    (Variables|/Script/Engine.CharacterMovementComponent|SetMaxWalkSpeed _charactermovement 426.0)))

(fn ConstructionScript)

(fn ShootRay
  (bind _muzzle (Variables|Default|GetMuzzle))
  (bind _returnvalue (Transformation|GetWorldLocation _muzzle))
  (bind (_outhit _returnvalue_2) (Collision|LineTraceByChannel _returnvalue (+ _returnvalue (* (Math|Vector|GetForwardVector _muzzle) 1e+04)) "TraceTypeQuery2" false 0 "ForOneFrame"))
  (return _outhit _returnvalue_2))