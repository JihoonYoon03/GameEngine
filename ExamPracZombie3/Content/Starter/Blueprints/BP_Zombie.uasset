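; BP_Zombie is an enemy character that pursues the Granny player and damages her when its capsule hits her.
; Each tick while alive, it records horizontal speed and calls Chase, which picks a fast or slow walk speed by distance, or no pursuit, then steers with AddMovementInput.
; Damage drains Health until it is flagged Dead and loses capsule collision.
; A separate Dissolve event destroys the actor.
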(event OnComponentHit(CapsuleComponent)
  (params (HitComponent :type Primitive%20Component%20Object%20Reference) (OtherActor :type Actor%20Object%20Reference) (OtherComp :type Primitive%20Component%20Object%20Reference) (NormalImpulse :type Vector :default "0, 0, 0") (Hit :type Hit%20Result%20Structure%20%28by%20ref%29))
  (bind _asgranny (Utilities|Casting|CastToGranny OtherActor))
  (Game|Damage|ApplyDamage _asgranny 1.0 0 0 "/Script/Engine.DamageType"))

(event Custom|Dissolve
  (Actor|SetLifeSpan 3.0)
  (Actor|DestroyActor))

(event EventBeginPlay)

(event Collision|EventActorBeginOverlap
  (params (OtherActor :type Actor%20Object%20Reference)))

(event EventTick
  (params (DeltaSeconds :type Float%20%28single-precision%29))
  (if (not (Variables|Default|GetDead))
    (Variables|Default|SetSpeed (Math|Vector|VectorLengthXY (Transformation|GetVelocity)))
    (bind (_found _location) (CallFunction|Chase))
    (if _found
      (Pawn|Input|AddMovementInput (Math|Vector|GetForwardVector (Math|Rotator|FindLookatRotation (Transformation|GetActorLocation) _location)) 1.0 false))))

(event Game|Damage|EventAnyDamage
  (params (Damage :type Float%20%28single-precision%29) (DamageType :type Damage%20Type%20Object%20Reference) (InstigatedBy :type Controller%20Object%20Reference) (DamageCauser :type Actor%20Object%20Reference))
  (bind _output_get (Variables|Default|SetHealth (- (Variables|Default|GetHealth) Damage)))
  (if (<= _output_get 0.0)
    (Variables|Default|SetDead true)
    (Collision|SetCollisionEnabled (Variables|Collision|GetCapsuleComponent) "NoCollision")))

(fn ConstructionScript)

(fn Chase
  (bind _charactermovement (Variables|Character|GetCharacterMovement))
  (bind _asgranny (Utilities|Casting|CastToGranny (Game|Player|GetPlayerPawn 0))
    (:then
      (if (Math|Float|InRange(Float) (Transformation|GetDistanceTo _asgranny) 0.0 1e+03)
        (Variables|/Script/Engine.CharacterMovementComponent|SetMaxWalkSpeed _charactermovement 257.0)
        (Variables|/Script/Engine.CharacterMovementComponent|SetbOrientRotationToMovement _charactermovement true :!label _label)
        (return true (Transformation|GetActorLocation _asgranny))
        (elif (Math|Float|InRange(Float) (Transformation|GetDistanceTo _asgranny) 1e+03 2.5e+03)
          (Variables|/Script/Engine.CharacterMovementComponent|SetMaxWalkSpeed _charactermovement 4e+01)
          (goto _label)
          (else
            _))))
    (:CastFailed
      _))
  (Variables|/Script/Engine.CharacterMovementComponent|SetbOrientRotationToMovement _charactermovement false)
  (return false "0, 0, 0"))