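; ZombieGamemode is a game mode that ends the game once no zombies remain and supports restarting the level.
; BeginPlay creates the death and clear widgets but neither stores them nor adds them to the viewport.
; Tick polls for all BP_Zombie actors every frame and quits the game when none are found.
; A RestartLevel event reloads the current level by name.
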(event Custom|Restart%20Level
  (bind _returnvalue (Game|GetCurrentLevelName true))
  (Game|OpenLevel(byName) (Utilities|String|StringToName _returnvalue)))

(event EventBeginPlay
  (UserInterface|CreateWidget "/Game/Starter/Blueprints/WBP_Death.WBP_Death_C")
  (UserInterface|CreateWidget "/Game/Starter/Blueprints/WBP_Clear.WBP_Clear_C"))

(event EventTick
  (params (DeltaSeconds :type Float%20%28single-precision%29))
  (bind _outactors (Actor|GetAllActorsOfClass "/Game/Starter/Blueprints/BP_Zombie.BP_Zombie_C"))
  (if (Utilities|Array|IsEmpty _outactors)
    (Game|QuitGame 0 "Quit" false)))

(fn ConstructionScript)