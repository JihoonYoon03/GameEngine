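; BP_Zombie is an enemy character that chases the Granny actor and deals damage when its capsule begins overlapping her.
; Each Tick updates Speed from horizontal velocity and, while alive, moves toward Granny via Chase, which sets a fast or slow walk speed by distance band.
; Incoming damage lowers Health, and reaching zero sets Dead and disables capsule collision.
; A separate Dissolve event destroys the actor.
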(event OnComponentBeginOverlap(CapsuleComponent)
  (params (OverlappedComponent :type Primitive%20Component%20Object%20Reference) (OtherActor :type Actor%20Object%20Reference) (OtherComp :type Primitive%20Component%20Object%20Reference) (OtherBodyIndex :type Integer) (bFromSweep :type Boolean) (SweepResult :type Hit%20Result%20Structure%20%28by%20ref%29))
  (bind _asgranny (Utilities|Casting|CastToGranny OtherActor))
  (Game|Damage|ApplyDamage _asgranny 1.0 0 0 "/Script/Engine.DamageType"))

(event Custom|Dissolve
  (Actor|SetLifeSpan 3.0)
  (Actor|DestroyActor))

(event EventBeginPlay)

(event Collision|EventActorBeginOverlap
  (params (OtherActor :type Actor%20Object%20Reference)))

(event EventTick
  (params (DeltaSeconds :type Float%20%28single-precision%29))
  (Variables|Default|SetSpeed (Math|Vector|VectorLengthXY (Transformation|GetVelocity)))
  (if (not (Variables|Default|GetDead?))
    (bind (_found _direction) (CallFunction|Chase))
    (if _found
      (Pawn|Input|AddMovementInput _direction 1.0 false))))

(event Game|Damage|EventAnyDamage
  (params (Damage :type Float%20%28single-precision%29) (DamageType :type Damage%20Type%20Object%20Reference) (InstigatedBy :type Controller%20Object%20Reference) (DamageCauser :type Actor%20Object%20Reference))
  (bind _output_get (Variables|Default|SetHealth (- (Variables|Default|GetHealth) Damage)))
  (if (<= _output_get 0.0)
    (Variables|Default|SetDead? true)
    (Collision|SetCollisionEnabled (Variables|Collision|GetCapsuleComponent) "NoCollision")))

(fn ConstructionScript)

(fn Chase
  (bind _charactermovement (Variables|Character|GetCharacterMovement))
  (bind _returnvalue (Actor|GetActorOfClass "/Game/Starter/Blueprints/Granny.Granny_C"))
  (Utilities|IsValid _returnvalue
    (:Is%20Valid
      (if (Math|Float|InRange(Float) (Transformation|GetDistanceTo _returnvalue) 0.0 1e+03)
        (Variables|/Script/Engine.CharacterMovementComponent|SetMaxWalkSpeed _charactermovement 257.0)
        (return true (Math|Vector|Normalize (- (Transformation|GetActorLocation _returnvalue) (Transformation|GetActorLocation))))
        (elif (Math|Float|InRange(Float) (Transformation|GetDistanceTo _returnvalue) 1e+03 2.5e+03)
          (Variables|/Script/Engine.CharacterMovementComponent|SetMaxWalkSpeed _charactermovement 4e+01)
          (return true (Math|Vector|Normalize (- (Transformation|GetActorLocation _returnvalue) (Transformation|GetActorLocation)))))))
    (:Is%20Not%20Valid
      (return false "0, 0, 0"))))