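; BP_HPGoldTrophy is a damageable trophy actor with a widget component showing a TrophyHP widget, presumably its health display.
; On BeginPlay it casts the component's widget to TrophyHP and passes itself in, giving the widget a reference to the actor.
; Any damage is subtracted from HP; at zero or below it spawns an explosion effect and sound at its location, then destroys itself.
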(event EventBeginPlay
  (|CallParentFunction)
  (bind _astrophy_hp (Utilities|Casting|CastToTrophyHP (UserInterface|GetWidget (Variables|Default|GetWidget%20Holding%20Component))))
  (Variables|/Game/Lec24-UMG/TrophyHP.TrophyHP_C|SetHPTrophy _astrophy_hp self))

(event Collision|EventActorBeginOverlap
  (params (OtherActor :type Actor%20Object%20Reference))
  (|CallParentFunction OtherActor) ; This node is disabled and will not be called.\nDrag off pins to build functionality.
)

(event EventTick
  (params (DeltaSeconds :type Float%20%28single-precision%29))
  (|CallParentFunction DeltaSeconds) ; This node is disabled and will not be called.\nDrag off pins to build functionality.
)

(event Game|Damage|EventAnyDamage
  (params (Damage :type Float%20%28single-precision%29) (DamageType :type Damage%20Type%20Object%20Reference) (InstigatedBy :type Controller%20Object%20Reference) (DamageCauser :type Actor%20Object%20Reference))
  (bind _returnvalue (Transformation|GetActorLocation))
  (bind _output_get (Variables|Default|SetHP (- (Variables|Default|GetHP) Damage)))
  (if (<= _output_get 0.0)
    (Effects|SpawnEmitteratLocation "/Game/StarterContent/Particles/P_Explosion.P_Explosion" _returnvalue "0, 0, 0" (Transformation|GetActorScale3D))
    (Audio|PlaySoundatLocation "/Game/StarterContent/Audio/Explosion01.Explosion01" _returnvalue "0, 0, 0" 1.0 1.0 0.0 0 0 0 0)
    (Actor|DestroyActor)))

(fn ConstructionScript
  (|CallParentFunction))