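; BP_Course is an actor that builds a straight course of rings toward CourseEnd, with coins along it.
; The Construction Script places evenly spaced, scaled ring meshes facing the course direction, plus about a thousand static mesh particles scattered randomly around the line.
; On BeginPlay it spawns BP_Coin actors at random points within a ring-scale spread, using world coordinates with a fixed height offset rather than the actor's transform.
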(event EventBeginPlay
  (bind _courseend (Variables|Default|GetCourseEnd))
  (bind _coursedirection (Variables|Default|GetCourseDirection))
  (bind _ringscale (Variables|Default|GetRingScale))
  (bind _returnvalue (Math|Vector|VectorLength _courseend))
  (bind _returnvalue_2 (Math|Conversions|RotationFromXVector _coursedirection))
  (bind _returnvalue_3 (* _ringscale 1e+02))
  (bind _returnvalue_4 (Math|Random|RandomFloatinRange 0.0 _returnvalue))
  (bind _returnvalue_5 (* _returnvalue_3 -1.0))
  (bind _returnvalue_6 (* _coursedirection _returnvalue_4))
  (for _index (range 0 (Variables|Default|GetCoins))
    (Game|SpawnActorfromClass "/Game/Blueprints/BP_Coin.BP_Coin_C" (Math|Transform|MakeTransform (Math|Vector|MakeVector (+ (.x _returnvalue_6) (Math|Random|RandomFloatinRange _returnvalue_5 _returnvalue_3)) (+ (.y _returnvalue_6) (Math|Random|RandomFloatinRange _returnvalue_5 _returnvalue_3)) (+ (+ (.z _returnvalue_6) (Math|Random|RandomFloatinRange _returnvalue_5 _returnvalue_3)) 1e+03)) (Math|Rotator|MakeRotator 0.0 (.pitch _returnvalue_2) (.yaw _returnvalue_2)) "1.000000,1.000000,1.000000") "Undefined" "MultiplyWithRoot" 0 0)))

(event Collision|EventActorBeginOverlap
  (params (OtherActor :type Actor%20Object%20Reference)))

(event EventTick
  (params (DeltaSeconds :type Float%20%28single-precision%29)))

(fn ConstructionScript
  (bind _courseend (Variables|Default|GetCourseEnd))
  (bind _particlespread (Variables|Default|GetParticleSpread))
  (bind _returnvalue (* _particlespread -1.0))
  (bind _output_get (Variables|Default|SetCourseDirection (Math|Vector|Normalize _courseend)))
  (for _index (range 0 (Math|Float|Truncate (Math|Float|SafeDivide (Math|Vector|VectorLength _courseend) (Math|Conversions|ToFloat(Integer) (* (Variables|Default|GetMeterPerRing) 100)))))
    (AddComponent|AddStaticMeshComponent false (Math|Transform|MakeTransform (* _index (* (Variables|Default|GetMeterPerRing) 100) _output_get) (Math|Rotator|MakeRotator 0.0 (.pitch (Math|Conversions|RotationFromXVector _output_get)) (.yaw (Math|Conversions|RotationFromXVector _output_get))) (Math|Conversions|ToVector(Float) (Variables|Default|GetRingScale)))))
  (for _index_2 (range 0 1000)
    (AddComponent|AddStaticMeshComponent false (Math|Transform|MakeTransform (Math|Vector|MakeVector (+ (.x (* (Variables|Default|GetCourseDirection) (Math|Random|RandomFloatinRange 0.0 (Math|Vector|VectorLength (Variables|Default|GetCourseEnd))))) (Math|Random|RandomFloatinRange _returnvalue _particlespread)) (+ (.y (* (Variables|Default|GetCourseDirection) (Math|Random|RandomFloatinRange 0.0 (Math|Vector|VectorLength (Variables|Default|GetCourseEnd))))) (Math|Random|RandomFloatinRange _returnvalue _particlespread)) (+ (.z (* (Variables|Default|GetCourseDirection) (Math|Random|RandomFloatinRange 0.0 (Math|Vector|VectorLength (Variables|Default|GetCourseEnd))))) (Math|Random|RandomFloatinRange _returnvalue _particlespread))) (Math|Rotator|MakeRotator 0.0 (.pitch (Math|Conversions|RotationFromXVector (Variables|Default|GetCourseDirection))) (.yaw (Math|Conversions|RotationFromXVector (Variables|Default|GetCourseDirection)))) "1.000000,1.000000,1.000000"))))