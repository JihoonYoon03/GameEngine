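; Player aircraft Blueprint that handles boosting, flight effects and distance reporting on top of a FloatingPawnMovement component.
; Each Tick adds the distance moved since the last frame to the WBP_UI meter.
; Holding LeftShift raises max speed and fades in a sound cue, while Tick spawns rear boost particles and decrements Fuel, with no empty check.
; Above a speed threshold, trail emitters spawn every frame at left and right arrows.
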(event EventBeginPlay
  (Variables|Default|SetLast%20Location (Transformation|GetActorLocation)))

(event Collision|EventActorBeginOverlap
  (params (OtherActor :type Actor%20Object%20Reference)))

(event EventTick
  (params (DeltaSeconds :type Float%20%28single-precision%29))
  (bind _returnvalue (Transformation|GetActorLocation))
  (bind _foundwidgets (Widget|GetAllWidgetsOfClass "/Game/Framework/WBP_UI.WBP_UI_C" true))
  (Default|AddMeter _foundwidgets (Math|Vector|VectorLength (- (Variables|Default|GetLast%20Location) _returnvalue)))
  (Variables|Default|SetLast%20Location _returnvalue)
  (if (Variables|Default|GetBoost?)
    (CallFunction|SpawnBoost))
  (if (Class|MovementComponent|IsExceedingMaxSpeed (Variables|Default|GetFloatingPawnMovement) 1e+04)
    (CallFunction|SpawnTrails)))

(event Input|KeyboardEvents|LeftShift
  (params (Key :type Key%20Structure :default "None"))
  (bind _floatingpawnmovement (Variables|Default|GetFloatingPawnMovement))
  (bind _boost_cue (Variables|Default|GetBoost_Cue))
  (:Pressed
    (Variables|Default|SetBoost? true)
    (Variables|/Script/Engine.FloatingPawnMovement|SetMaxSpeed _floatingpawnmovement 2e+04)
    (Audio|Components|Audio|FadeIn _boost_cue 0.0 1.0 0.0 "Linear" :!class /Script/Engine.AudioComponent))
  (:Released
    (Variables|Default|SetBoost? false)
    (Variables|/Script/Engine.FloatingPawnMovement|SetMaxSpeed _floatingpawnmovement 1.2e+04)
    (Audio|Components|Audio|FadeOut _boost_cue 0.0 0.0 "Linear" :!class /Script/Engine.AudioComponent)))

(fn ConstructionScript)

(fn SpawnTrails
  (bind _arrowl (Variables|Default|GetArrowL))
  (bind _arrowr (Variables|Default|GetArrowR))
  (Effects|SpawnEmitteratLocation "/Game/Assets/P_Trail.P_Trail" (Transformation|GetWorldLocation _arrowl) (Transformation|GetWorldRotation _arrowl) "0.300000,0.300000,0.300000")
  (Effects|SpawnEmitteratLocation "/Game/Assets/P_Trail.P_Trail" (Transformation|GetWorldLocation _arrowr) (Transformation|GetWorldRotation _arrowr) "0.300000,0.300000,0.300000"))

(fn SpawnBoost
  (bind _arrowback (Variables|Default|GetArrowBack))
  (Effects|SpawnEmitteratLocation "/Game/Assets/P_Boost.P_Boost" (Transformation|GetWorldLocation _arrowback) (Transformation|GetWorldRotation _arrowback))
  (Math|Float|DecrementFloat (Variables|Default|GetFuel)))