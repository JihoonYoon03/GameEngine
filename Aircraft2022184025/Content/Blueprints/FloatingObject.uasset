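; FloatingObject is a component-style Blueprint that makes its owning actor bob up and down.
; BeginPlay caches the owner and adds random variation to Frequency and Amplitude so that instances move differently.
; Tick adds a sine-of-game-time Z world offset each frame, so motion accumulates and depends on frame rate.
; StartLocation is recorded at BeginPlay but never used in the movement.
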(event EventBeginPlay
  (bind _output_get (Variables|Default|SetParent (Components|GetOwner)))
  (Variables|Default|SetStart%20Location (Transformation|GetActorLocation _output_get))
  (Variables|Default|SetFrequency (+ (Variables|Default|GetFrequency) (Math|Random|RandomFloatinRange 0.0 1.0)))
  (Variables|Default|SetAmplitude (+ (Variables|Default|GetAmplitude) (Math|Random|RandomFloatinRange 0.0 1e+01))))

(event EventTick
  (params (DeltaSeconds :type Float%20%28single-precision%29))
  (Transformation|AddActorWorldOffset (Variables|Default|GetParent) (Math|Vector|MakeVector 0.0 0.0 (* (Math|Trig|Sin(Radians) (* (Variables|Default|GetFrequency) 3.141592 (Utilities|Time|GetTimeSeconds))) (Variables|Default|GetAmplitude)))))