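; BP_Ball is a thrown projectile that deals Frozen-type damage to whatever it hits.
; Stick halts its movement and collision, while Release launches it toward a target point on a suggested arc with distance-scaled, clamped speed, or straight at fixed speed if no arc is found.
; Collision re-enables shortly after release; on hit it spawns burst effects aligned to launch direction, plays a sound and destroys itself.
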(event OnComponentHit(StaticMeshComponent)
  (params (HitComponent :type Primitive%20Component%20Object%20Reference) (OtherActor :type Actor%20Object%20Reference) (OtherComp :type Primitive%20Component%20Object%20Reference) (NormalImpulse :type Vector :default "0, 0, 0") (Hit :type Hit%20Result%20Structure%20%28by%20ref%29))
  (bind _returnvalue (Transformation|GetActorLocation))
  (bind _spawnvelocity (Variables|Default|GetSpawnVelocity))
  (bind _returnvalue_2 (Math|Vector|Normalize _spawnvelocity))
  (bind _returnvalue_3 (Math|Conversions|RotationFromXVector _returnvalue_2))
  (Game|Damage|ApplyDamage OtherActor 1.0 0 0 "/Game/_TEST3/Frozen.Frozen_C")
  (Niagara|SpawnSystematLocation "/Niagara/DefaultAssets/Templates/Systems/DirectionalBurst.DirectionalBurst" _returnvalue _returnvalue_3)
  (Niagara|SpawnSystematLocation "/Niagara/DefaultAssets/Templates/Systems/DirectionalBurstLightweight.DirectionalBurstLightweight" _returnvalue _returnvalue_3)
  (Audio|PlaySoundatLocation "/Engine/VREditor/Sounds/UI/Foliage_Placed.Foliage_Placed" _returnvalue "0, 0, 0" 1.0 1.0 0.0 0 0 0 0)
  (Actor|DestroyActor))

(event EventBeginPlay)

(event Collision|EventActorBeginOverlap
  (params (OtherActor :type Actor%20Object%20Reference)))

(event EventTick
  (params (DeltaSeconds :type Float%20%28single-precision%29)))

(event EventRelease
  (params (From :type Vector :default "0, 0, 0") (To :type Vector :default "0, 0, 0"))
  (bind _returnvalue (- To From))
  (bind _projectilemovement (Variables|Default|GetProjectileMovement))
  (bind _returnvalue_2 (Math|Vector|Normalize _returnvalue))
  (bind _returnvalue_3 (* _returnvalue_2 2e+03))
  (bind (_tossvelocity _returnvalue_4) (Class|GameplayStatics|BlueprintSuggestProjectileVelocity From To (Math|Float|Clamp(Float) (Math|Vector|Distance(Vector) From To) 2e+02 2e+03) 0.0 "DoNotTrace" 0.0 false true false))
  (if _returnvalue_4
    (Variables|Default|SetSpawnVelocity _tossvelocity)
    (Variables|/Script/Engine.MovementComponent|SetVelocity _projectilemovement _tossvelocity)
    (else
      (Variables|Default|SetSpawnVelocity _returnvalue_3)
      (Variables|/Script/Engine.MovementComponent|SetVelocity _projectilemovement _returnvalue_3)))
  (Components|Activation|Activate _projectilemovement true)
  (Utilities|FlowControl|Delay 0.1)
  (Collision|SetActorEnableCollision true))

(fn ConstructionScript)

(fn Stick
  (Components|Activation|Deactivate (Variables|Default|GetProjectileMovement))
  (Collision|SetActorEnableCollision false)
  (return true))