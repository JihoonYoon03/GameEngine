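; Zombie character that moves toward a supplied location, melees at close range and can be frozen, then shattered.
; Chase plays a DoOnce-gated attack montage whose notifies open the window in which Attack overlaps send HitMessage to the other actor.
; Frozen-type damage stops movement and animation, applies an ice overlay and blocks Chase.
; A Hit while frozen spawns a burst effect and sound, then destroys the zombie.
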(event OnComponentBeginOverlap(Attack)
  (params (OverlappedComponent :type Primitive%20Component%20Object%20Reference) (OtherActor :type Actor%20Object%20Reference) (OtherComp :type Primitive%20Component%20Object%20Reference) (OtherBodyIndex :type Integer) (bFromSweep :type Boolean) (SweepResult :type Hit%20Result%20Structure%20%28by%20ref%29))
  (if (Variables|Default|GetHitable)
    (Class|HitInterface|Hit(Message) OtherActor)))

(event EventBeginPlay)

(event Collision|EventActorBeginOverlap
  (params (OtherActor :type Actor%20Object%20Reference)))

(event EventTick
  (params (DeltaSeconds :type Float%20%28single-precision%29))
  (if (not (Variables|Default|GetFrozen))
    (Variables|Default|SetSpeed (Math|Vector|VectorLengthXY (Transformation|GetVelocity)))))

(event EventChase
  (params (Location :type Vector :default "0, 0, 0"))
  (bind _returnvalue (Transformation|GetActorLocation))
  (bind _returnvalue_2 (- Location _returnvalue))
  (if (not (Variables|Default|GetFrozen))
    (Pawn|Input|AddMovementInput (Math|Vector|Normalize _returnvalue_2) 1.0 false)
    (if (<= (Math|Vector|VectorLength _returnvalue_2) 2e+02)
      (Utilities|FlowControl|DoOnce false :!label _label
        (:Completed
          (bind _notifyname (Animation|Montage|PlayMontage (Variables|Character|GetMesh) "/Game/Characters/Zombie/Animations/ZombieMontage.ZombieMontage" 1.0 0.0 "Default")
            (:OnCompleted
              (goto _label Reset))
            (:OnNotifyBegin
              (switch name _notifyname
                (:HitStart
                  (Variables|Default|SetHitable true))
                (:HitEnd
                  (Variables|Default|SetHitable false))))))))))

(event Game|Damage|EventAnyDamage
  (params (Damage :type Float%20%28single-precision%29) (DamageType :type Damage%20Type%20Object%20Reference) (InstigatedBy :type Controller%20Object%20Reference) (DamageCauser :type Actor%20Object%20Reference))
  (Utilities|Casting|CastToFrozen DamageType)
  (Components|Movement|StopMovementImmediately (Variables|Character|GetCharacterMovement))
  (Variables|/Script/Engine.SkeletalMeshComponent|SetGlobalAnimRateScale (Variables|Character|GetMesh) 0.0)
  (Rendering|Material|SetOverlayMaterial (Variables|Character|GetMesh) "/Game/_TEST3/M_Frozen.M_Frozen" :!class /Script/Engine.MeshComponent)
  (Variables|Default|SetFrozen true))

(event EventHit
  (bind _returnvalue (Transformation|GetActorLocation))
  (if (Variables|Default|GetFrozen)
    (Niagara|SpawnSystematLocation "/Niagara/DefaultAssets/Templates/Systems/RadialBurst.RadialBurst" _returnvalue "0, 0, 0" "2.000000,2.000000,2.000000")
    (Audio|PlaySoundatLocation "/Engine/VREditor/Sounds/UI/Flashlight_Switch.Flashlight_Switch" _returnvalue "0, 0, 0" 1.0 2.0 0.0 0 0 0 0)
    (Actor|DestroyActor)))

(fn ConstructionScript)