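; BP_Aircraft is an aircraft with a Shift-held afterburner boost and a travelled-distance counter.
; Each tick it finds the WBP_UI widgets and feeds the distance moved since last frame to AddMeter.
; Left Shift sets Boost, switches FloatingPawnMovement's max speed and fades the afterburner sound.
; Tick spawns afterburner emitters at the rear arrow while boosting, and stream emitters at the left and right arrows above a speed threshold.
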(event EventBeginPlay
  (Variables|Default|SetLast%20Location (Transformation|GetActorLocation)))

(event Collision|EventActorBeginOverlap
  (params (OtherActor :type Actor%20Object%20Reference)))

(event EventTick
  (params (DeltaSeconds :type Float%20%28single-precision%29))
  (bind _returnvalue (Transformation|GetActorLocation))
  (bind _foundwidgets (Widget|GetAllWidgetsOfClass "/Game/Frameworks/WBP_UI.WBP_UI_C" true))
  (Default|AddMeter _foundwidgets (Math|Vector|VectorLength (- (Variables|Default|GetLast%20Location) _returnvalue)))
  (Variables|Default|SetLast%20Location _returnvalue)
  (if (Variables|Default|GetBoost?)
    (CallFunction|SpawnAfterBurner))
  (if (Class|MovementComponent|IsExceedingMaxSpeed (Variables|Default|GetFloatingPawnMovement) 1e+04)
    (CallFunction|SpawnStream)))

(event Input|KeyboardEvents|LeftShift
  (params (Key :type Key%20Structure :default "None"))
  (bind _afterburner_cue (Variables|Default|GetAfterBurner_Cue))
  (bind _floatingpawnmovement (Variables|Default|GetFloatingPawnMovement))
  (:Pressed
    (Variables|Default|SetBoost? true)
    (Variables|/Script/Engine.FloatingPawnMovement|SetMaxSpeed _floatingpawnmovement 2e+04)
    (Audio|Components|Audio|FadeIn _afterburner_cue 0.2 1.0 0.0 "Linear" :!class /Script/Engine.AudioComponent))
  (:Released
    (Variables|Default|SetBoost? false)
    (Variables|/Script/Engine.FloatingPawnMovement|SetMaxSpeed _floatingpawnmovement 1.2e+04)
    (Audio|Components|Audio|FadeOut _afterburner_cue 0.5 0.0 "Linear" :!class /Script/Engine.AudioComponent)))

(fn ConstructionScript)

(fn SpawnStream
  (bind _arrowr (Variables|Default|GetArrowR))
  (bind _arrowl (Variables|Default|GetArrowL))
  (Effects|SpawnEmitteratLocation "/Game/Assets/P_AircraftStream.P_AircraftStream" (Transformation|GetWorldLocation _arrowl) (Math|Conversions|RotationFromXVector (Math|Vector|GetForwardVector _arrowl)) "0.200000,0.200000,0.200000")
  (Effects|SpawnEmitteratLocation "/Game/Assets/P_AircraftStream.P_AircraftStream" (Transformation|GetWorldLocation _arrowr) (Math|Conversions|RotationFromXVector (Math|Vector|GetForwardVector _arrowr)) "0.200000,0.200000,0.200000"))

(fn SpawnAfterBurner
  (bind _arrowback (Variables|Default|GetArrowBack))
  (Effects|SpawnEmitteratLocation "/Game/Assets/P_AfterBurner.P_AfterBurner" (Transformation|GetWorldLocation _arrowback) (Math|Conversions|RotationFromXVector (Math|Vector|GetForwardVector _arrowback))))