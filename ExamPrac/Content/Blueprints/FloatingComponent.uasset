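; FloatingComponent is a component that makes its owning actor bob up and down.
; On BeginPlay it caches the owner and picks a random frequency and amplitude, so each instance moves differently.
; Each Tick adds a sine of game time as a vertical world offset, accumulating per frame without delta-time scaling.
; The saved start location is not used in the motion.
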(event EventBeginPlay
  (bind _output_get (Variables|Default|SetParent (Components|GetOwner)))
  (Variables|Default|SetStartLocation (Transformation|GetActorLocation _output_get))
  (Variables|Default|SetFrequency (Math|Random|RandomFloatinRange 2.0 4.0))
  (Variables|Default|SetAmplitude (Math|Random|RandomFloatinRange 15.0 3e+01)))

(event EventTick
  (params (DeltaSeconds :type Float%20%28single-precision%29))
  (Transformation|AddActorWorldOffset (Variables|Default|GetParent) (Math|Vector|MakeVector 0.0 0.0 (* (Math|Trig|Sin(Radians) (* (Variables|Default|GetFrequency) 3.141592 (Utilities|Time|GetTimeSeconds))) (Variables|Default|GetAmplitude)))))