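; BP_Course is a course actor that lays a straight line of ring meshes toward CourseEnd and scatters coins along it.
; The construction script normalizes CourseEnd into CourseDirection, then adds scaled static mesh rings at MeterPerRing intervals, oriented along it.
; BeginPlay spawns BP_Coin actors in a MaxCoins loop, at random distances along that direction with per-axis jitter scaled by RingScale, without adding the actor's location.
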(event EventBeginPlay
  (bind _courseend (Variables|Default|GetCourseEnd))
  (bind _coursedirection (Variables|Default|GetCourseDirection))
  (bind _returnvalue (Math|Conversions|RotationFromXVector _coursedirection))
  (bind _returnvalue_2 (Math|Vector|VectorLength _courseend))
  (bind _returnvalue_3 (Math|Random|RandomFloatinRange 0.0 _returnvalue_2))
  (bind _returnvalue_4 (* _coursedirection _returnvalue_3))
  (for _index (range 0 (Variables|Default|GetMaxCoins))
    (Game|SpawnActorfromClass "/Game/Blueprints/BP_Coin.BP_Coin_C" (Math|Transform|MakeTransform (Math|Vector|MakeVector (+ (.x _returnvalue_4) (CallFunction|RandomFloatbyScale)) (+ (.y _returnvalue_4) (CallFunction|RandomFloatbyScale)) (+ (.z _returnvalue_4) (CallFunction|RandomFloatbyScale))) (Math|Rotator|MakeRotator 0.0 (.pitch _returnvalue) (.yaw _returnvalue)) "1.000000,1.000000,1.000000") "Undefined" "MultiplyWithRoot" 0 0)))

(event Collision|EventActorBeginOverlap
  (params (OtherActor :type Actor%20Object%20Reference)))

(event EventTick
  (params (DeltaSeconds :type Float%20%28single-precision%29)))

(fn ConstructionScript
  (bind _courseend (Variables|Default|GetCourseEnd))
  (bind _output_get (Variables|Default|SetCourseDirection (Math|Vector|Normalize _courseend)))
  (for _index (range 0 (Math|Float|Truncate (Math|Float|SafeDivide (Math|Vector|VectorLength _courseend) (* (Variables|Default|GetMeterPerRing) 1e+02))))
    (AddComponent|AddStaticMeshComponent false (Math|Transform|MakeTransform (* _index (* (Variables|Default|GetMeterPerRing) 1e+02) _output_get) (Math|Rotator|MakeRotator 0.0 (.pitch (Math|Conversions|RotationFromXVector _output_get)) (.yaw (Math|Conversions|RotationFromXVector _output_get))) (Math|Conversions|ToVector(Float) (Variables|Default|GetRingScale))))))

(fn RandomFloatbyScale
  (bind _ringscale (Variables|Default|GetRingScale))
  (return (Math|Random|RandomFloatinRange (* _ringscale -5e+02) (* _ringscale 5e+02))))