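; Actor component that makes its owning actor bob up and down.
; On begin play it stores the owner's location, then each tick offsets Z from that point by a sine of game time scaled by Frequency and Amplitude.
; Turn On re-captures the current location as the center and enables ticking, while Turn Off disables ticking.
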(event EventBeginPlay
  (bind _output_get (Variables|Default|SetParentActor (Components|GetOwner)))
  (Variables|Default|SetStartLocation (Transformation|GetActorLocation _output_get)))

(event EventTick
  (params (DeltaSeconds :type Float%20%28single-precision%29))
  (Transformation|SetActorLocation (Variables|Default|GetParentActor) (+ (Variables|Default|GetStartLocation) (Math|Vector|MakeVector 0.0 0.0 (* (Math|Trig|Sin(Radians) (* (Utilities|Time|GetTimeSeconds) 3.141592 (Variables|Default|GetFrequency))) (Variables|Default|GetAmplitude)))) false false))

(fn Turnon
  (Variables|Default|SetStartLocation (Transformation|GetActorLocation (Variables|Default|GetParentActor)))
  (Components|Tick|SetComponentTickEnabled true))

(fn TurnOff
  (Components|Tick|SetComponentTickEnabled false))