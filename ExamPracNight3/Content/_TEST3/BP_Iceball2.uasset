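; BP_Iceball2 is an ice projectile that waits inert after spawning until Release launches it with a given velocity.
; Release activates projectile movement, then enables collision after a short delay.
; On a hit it applies Frozen damage, plays burst particle effects oriented along the launch velocity plus a sound, then destroys itself.
; A separate Stick function halts movement and disables collision.
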(event OnComponentHit(StaticMesh)
  (params (HitComponent :type Primitive%20Component%20Object%20Reference) (OtherActor :type Actor%20Object%20Reference) (OtherComp :type Primitive%20Component%20Object%20Reference) (NormalImpulse :type Vector :default "0, 0, 0") (Hit :type Hit%20Result%20Structure%20%28by%20ref%29))
  (bind _spawnvelocity (Variables|Default|GetSpawnVelocity))
  (bind _returnvalue (Math|Vector|Normalize _spawnvelocity))
  (bind _returnvalue_2 (Math|Conversions|RotationFromXVector _returnvalue))
  (if (not (Variables|Default|GetSpawned))
    (Game|Damage|ApplyDamage OtherActor 1.0 0 0 "/Game/_TEST3/Frozen.Frozen_C")
    (Niagara|SpawnSystematLocation "/Niagara/DefaultAssets/Templates/Systems/DirectionalBurst.DirectionalBurst" (.location Hit) _returnvalue_2)
    (Niagara|SpawnSystematLocation "/Niagara/DefaultAssets/Templates/Systems/DirectionalBurstLightweight.DirectionalBurstLightweight" (.location Hit) _returnvalue_2)
    (Audio|PlaySoundatLocation "/Engine/VREditor/Sounds/UI/Foliage_Placed.Foliage_Placed" (.location Hit) "0, 0, 0" 0.9 1.2 0.0 0 0 0 0)
    (Actor|DestroyActor)))

(event EventBeginPlay
  (Variables|Default|SetSpawned true))

(event Collision|EventActorBeginOverlap
  (params (OtherActor :type Actor%20Object%20Reference)))

(event EventTick
  (params (DeltaSeconds :type Float%20%28single-precision%29)))

(event EventRelease
  (params (Velocity :type Vector :default "0, 0, 0"))
  (bind _projectilemovement (Variables|Default|GetProjectileMovement))
  (bind _output_get (Variables|Default|SetSpawnVelocity Velocity))
  (Variables|/Script/Engine.MovementComponent|SetVelocity _projectilemovement _output_get)
  (Components|Activation|Activate _projectilemovement true)
  (Variables|Default|SetSpawned false)
  (Utilities|FlowControl|Delay 0.1)
  (Collision|SetActorEnableCollision true))

(fn ConstructionScript)

(fn Stick
  (Components|Activation|Deactivate (Variables|Default|GetProjectileMovement))
  (Collision|SetActorEnableCollision false)
  (return true))