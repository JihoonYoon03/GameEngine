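; BP_Ball is a throwable projectile that deals Frozen damage to what it hits, then destroys itself with burst effects and a sound.
; Stick deactivates projectile movement and collision.
; Release applies a given velocity, activates movement, then re-enables collision and clears the Spawned flag after a short delay.
; Sphere hits are ignored while Spawned is set, and the bursts are oriented along the launch velocity.
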(event OnComponentHit(Sphere)
  (params (HitComponent :type Primitive%20Component%20Object%20Reference) (OtherActor :type Actor%20Object%20Reference) (OtherComp :type Primitive%20Component%20Object%20Reference) (NormalImpulse :type Vector :default "0, 0, 0") (Hit :type Hit%20Result%20Structure%20%28by%20ref%29))
  (bind _returnvalue (Transformation|GetActorLocation))
  (bind _spawnvelocity (Variables|Default|GetSpawnVelocity))
  (bind _returnvalue_2 (Math|Conversions|RotationFromXVector _spawnvelocity))
  (if (not (Variables|Default|GetSpawned))
    (Game|Damage|ApplyDamage OtherActor 1.0 0 0 "/Game/_TEST3/Frozen.Frozen_C")
    (Niagara|SpawnSystematLocation "/Niagara/DefaultAssets/Templates/Systems/DirectionalBurst.DirectionalBurst" _returnvalue _returnvalue_2)
    (Niagara|SpawnSystematLocation "/Niagara/DefaultAssets/Templates/Systems/DirectionalBurstLightweight.DirectionalBurstLightweight" _returnvalue _returnvalue_2)
    (Audio|PlaySoundatLocation "/Engine/VREditor/Sounds/UI/Foliage_Placed.Foliage_Placed" _returnvalue "0, 0, 0" 1.0 1.0 0.0 0 0 0 0)
    (Actor|DestroyActor)))

(event EventBeginPlay
  (Variables|Default|SetSpawned true))

(event Collision|EventActorBeginOverlap
  (params (OtherActor :type Actor%20Object%20Reference)))

(event EventTick
  (params (DeltaSeconds :type Float%20%28single-precision%29)))

(event EventRelease
  (params (Velocity :type Vector :default "0, 0, 0"))
  (bind _projectilemovement (Variables|Default|GetProjectileMovement))
  (bind _output_get (Variables|Default|SetSpawnVelocity Velocity))
  (Variables|/Script/Engine.MovementComponent|SetVelocity _projectilemovement _output_get)
  (Components|Activation|Activate _projectilemovement true)
  (Utilities|FlowControl|Delay 0.1)
  (Collision|SetActorEnableCollision true)
  (Variables|Default|SetSpawned false))

(fn ConstructionScript)

(fn Stick
  (Components|Activation|Deactivate (Variables|Default|GetProjectileMovement))
  (Collision|SetActorEnableCollision false)
  (return true))