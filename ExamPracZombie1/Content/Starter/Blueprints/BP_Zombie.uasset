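; Zombie enemy character that chases the player and dies when its health runs out.
; Each living tick it records its ground speed and moves along the yaw toward player 0, with TracePlayer setting fast, slow or zero walk speed by distance band.
; Lethal damage sets Dead and disables capsule collision; FinishDeath destroys the actor.
; Wander is an uncalled stub with constant conditions.
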(event Custom|FinishDeath
  (Actor|SetLifeSpan 3.0)
  (Actor|DestroyActor))

(event EventBeginPlay
  (Variables|Default|SetToPlayer "0, 0, 0"))

(event Collision|EventActorBeginOverlap
  (params (OtherActor :type Actor%20Object%20Reference)))

(event EventTick
  (params (DeltaSeconds :type Float%20%28single-precision%29))
  (if (not (Variables|Default|GetDead))
    (Variables|Default|SetSpeed (Math|Vector|VectorLengthXY (Transformation|GetVelocity)))
    (bind _found (CallFunction|TracePlayer))
    (if _found
      (Pawn|Input|AddMovementInput (Math|Vector|GetForwardVector (Variables|Default|GetToPlayer)) 1.0 false))))

(event Game|Damage|EventAnyDamage
  (params (Damage :type Float%20%28single-precision%29) (DamageType :type Damage%20Type%20Object%20Reference) (InstigatedBy :type Controller%20Object%20Reference) (DamageCauser :type Actor%20Object%20Reference))
  (bind _output_get (Variables|Default|SetHealth (- (Variables|Default|GetHealth) Damage)))
  (if (<= _output_get 0.0)
    (Variables|Default|SetDead true)
    (Collision|SetCollisionEnabled (Variables|Collision|GetCapsuleComponent) "NoCollision")))

(fn ConstructionScript)

(fn TracePlayer
  (bind _returnvalue (Game|GetPlayerCharacter 0))
  (bind _charactermovement (Variables|Character|GetCharacterMovement))
  (bind _returnvalue_2 (Transformation|GetDistanceTo _returnvalue))
  (if (Utilities|IsValid _returnvalue)
    (Variables|Default|SetToPlayer (Math|Rotator|MakeRotator 0.0 0.0 (.yaw (Math|Rotator|FindLookatRotation (Transformation|GetActorLocation) (Transformation|GetActorLocation _returnvalue)))))
    (if (Math|Float|InRange(Float) _returnvalue_2 0.0 1e+03)
      (Variables|/Script/Engine.CharacterMovementComponent|SetMaxWalkSpeed _charactermovement 257.0)
      (elif (Math|Float|InRange(Float) _returnvalue_2 1e+03 2e+03)
        (Variables|/Script/Engine.CharacterMovementComponent|SetMaxWalkSpeed _charactermovement 4e+01)
        (else
          (Variables|/Script/Engine.CharacterMovementComponent|SetMaxWalkSpeed _charactermovement 0.0))))
    (return true)
    (else
      (return false))))

(fn Wander
  (if (< 0.0 6.0)
    (Pawn|Input|AddMovementInput (Transformation|GetActorForwardVector) 1.0 false)
    (elif true
      (if (not (> 0.0 1e+01))
        (Transformation|SetActorRotation (Math|Interpolation|RInterpTo (Transformation|GetActorRotation) "0, 0, 0" (Utilities|Time|GetTimeSeconds) 0.001))))))