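; Player character Granny: moves relative to camera, sprints, jumps, and picks up a rifle to aim and shoot.
; Right mouse toggles over-the-shoulder aiming with slower walk and montage; left fires a muzzle trace that spawns an explosion and applies damage.
; Tick updates Speed and, while aiming, draws that trace as debug.
; When Ejected, Space near ground sets Landing, otherwise landing kills her; Restart reloads the level.
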(event Custom|Pick%20Weapon
  (Variables|Default|SetGot%20Weapon? true)
  (Rendering|SetVisibility (Variables|Default|GetRifle) true false)
  (Audio|PlaySoundatLocation "/Engine/VREditor/Sounds/UI/Camera_Shutter.Camera_Shutter" (Transformation|GetActorLocation) "0, 0, 0" 1.0 1.0 0.0 0 0 0 0))

(event Custom|Restart
  (bind _returnvalue (Game|GetCurrentLevelName true))
  (Game|OpenLevel(byName) (Utilities|String|StringToName _returnvalue)))

(event Input|EnhancedActionEvents|EnhancedInputActionIA_MoveGranny
  (params (ActionValue :type Vector%202D%20Structure) (ElapsedSeconds :type Float%20%28double-precision%29) (TriggeredSeconds :type Float%20%28double-precision%29) (InputAction :type Input%20Action%20Object%20Reference :default "/Game/Starter/Assets/Inputs/IA_MoveGranny.IA_MoveGranny"))
  (bind _returnvalue (Pawn|GetControlRotation :!class /Script/Engine.Pawn))
  ;[0.15 0.15 0.15 0.5] RPG Style
  (Pawn|Input|AddMovementInput (Math|Vector|GetForwardVector (Math|Rotator|MakeRotator 0.0 0.0 (.yaw _returnvalue))) (.x ActionValue) false)
  (Pawn|Input|AddMovementInput (Math|Vector|GetRightVector (Math|Rotator|MakeRotator 0.0 0.0 (.yaw _returnvalue))) (.y ActionValue) false))

(event Input|EnhancedActionEvents|EnhancedInputActionIA_JumpGranny
  (params (ActionValue :type Boolean) (ElapsedSeconds :type Float%20%28double-precision%29) (TriggeredSeconds :type Float%20%28double-precision%29) (InputAction :type Input%20Action%20Object%20Reference :default "/Game/Starter/Assets/Inputs/IA_JumpGranny.IA_JumpGranny"))
  (:Started
    (Character|Jump)))

(event EventBeginPlay)

(event Collision|EventActorBeginOverlap
  (params (OtherActor :type Actor%20Object%20Reference)))

(event EventTick
  (params (DeltaSeconds :type Float%20%28single-precision%29))
  (Variables|Default|SetSpeed (Math|Vector|VectorLengthXY (Transformation|GetVelocity)))
  (CallFunction|ShootRayfromMuzzle))

(event EventOnLanded
  (params (Hit :type Hit%20Result%20Structure%20%28by%20ref%29))
  (if (Variables|Default|GetEjected?)
    (if (not (Variables|Default|GetLanding?))
      (Variables|Default|SetDead? true)
      (Input|DisableInput 0))))

(event Input|MouseEvents|RightMouseButton
  (params (Key :type Key%20Structure :default "None"))
  (bind _springarm (Variables|Default|GetSpringArm))
  (bind _camera (Variables|Default|GetCamera))
  (bind _charactermovement (Variables|Character|GetCharacterMovement))
  (bind _got_weapon_ (Variables|Default|GetGot%20Weapon?))
  (:Pressed
    (if _got_weapon_
      (Variables|Default|SetAiming? true)
      (Variables|/Script/Engine.SpringArmComponent|SetTargetArmLength _springarm 1.5e+02)
      (Transformation|SetRelativeLocation _camera "0.000000,70.000000,50.000000" false false)
      (Variables|Default|SetbUseControllerRotationYaw true)
      (Variables|/Script/Engine.CharacterMovementComponent|SetbOrientRotationToMovement _charactermovement false)
      (Variables|/Script/Engine.CharacterMovementComponent|SetMaxWalkSpeed _charactermovement 1.5e+02)
      (Animation|Montage|PlayMontage (Variables|Character|GetMesh) "/Game/Starter/Assets/Granny/Animations/ComboAttackMontage.ComboAttackMontage" 1.0 0.0 "AimingIdle")))
  (:Released
    (if _got_weapon_
      (Variables|Default|SetAiming? false)
      (Variables|/Script/Engine.SpringArmComponent|SetTargetArmLength _springarm 3e+02)
      (Transformation|SetRelativeLocation _camera "0, 0, 0" false false)
      (Variables|Default|SetbUseControllerRotationYaw false)
      (Variables|/Script/Engine.CharacterMovementComponent|SetbOrientRotationToMovement _charactermovement true)
      (Variables|/Script/Engine.CharacterMovementComponent|SetMaxWalkSpeed _charactermovement 426.0)
      (Animation|StopAnimMontage "/Game/Starter/Assets/Granny/Animations/ComboAttackMontage.ComboAttackMontage"))))

(event Input|MouseEvents|LeftMouseButton
  (params (Key :type Key%20Structure :default "None"))
  (:Pressed
    (if (Variables|Default|GetAiming?)
      (Animation|Montage|PlayMontage (Variables|Character|GetMesh) "/Game/Starter/Assets/Granny/Animations/ComboAttackMontage.ComboAttackMontage" 1.0 0.0 "Fire"
        (:then
          (bind (_hit_ _result) (CallFunction|ShootRayfromMuzzle))
          (if _hit_
            (Effects|SpawnEmitteratLocation "/Game/StarterContent/Particles/P_Explosion.P_Explosion" (.location _result) "0, 0, 0" "0.500000,0.500000,0.500000")
            (Game|Damage|ApplyDamage (.hitactor _result) 1e+02 0 0 "/Script/Engine.DamageType")))))))

(event Input|KeyboardEvents|SpaceBar
  (params (Key :type Key%20Structure :default "None"))
  (bind _returnvalue (Transformation|GetActorLocation))
  (:Pressed
    (if (Variables|Default|GetEjected?)
      (bind (_outhit _returnvalue_2) (Collision|LineTraceByChannel _returnvalue (- _returnvalue "0.000000,0.000000,5000.000000") "TraceTypeQuery1" false 0 "None"))
      (if _returnvalue_2
        (if (< (.distance _outhit) 2e+03)
          (Variables|Default|SetLanding? true))))))

(event Input|KeyboardEvents|LeftShift
  (params (Key :type Key%20Structure :default "None"))
  (bind _charactermovement (Variables|Character|GetCharacterMovement))
  (:Pressed
    (Variables|/Script/Engine.CharacterMovementComponent|SetMaxWalkSpeed _charactermovement 852.0))
  (:Released
    (Variables|/Script/Engine.CharacterMovementComponent|SetMaxWalkSpeed _charactermovement 426.0)))

(fn ConstructionScript)

(fn ShootRayfromMuzzle
  (bind _muzzle (Variables|Default|GetMuzzle))
  (bind _returnvalue (Transformation|GetWorldLocation _muzzle))
  (if (Variables|Default|GetAiming?)
    (bind (_outhit _returnvalue_2) (Collision|LineTraceByChannel _returnvalue (+ _returnvalue (* (Math|Vector|GetForwardVector _muzzle) 1e+04)) "TraceTypeQuery2" false 0 "ForOneFrame"))
    (return _returnvalue_2 _outhit)))