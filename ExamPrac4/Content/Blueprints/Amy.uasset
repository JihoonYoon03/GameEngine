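; Amy is a player-controlled Character with movement, jumping, a punch combo and a wave.
; Enhanced Input moves her relative to control yaw and triggers jumps, while Tick stores horizontal velocity as Speed.
; Left click plays ComboAction montage sections LPunch then RPunch on blend out, with a DoOnce blocking re-entry until the chain ends.
; Holding H plays the Waving section and blocks new punches; releasing it stops the montage.
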(event Input|EnhancedActionEvents|EnhancedInputActionIA_MoveAmy
  (params (ActionValue :type Vector%202D%20Structure) (ElapsedSeconds :type Float%20%28double-precision%29) (TriggeredSeconds :type Float%20%28double-precision%29) (InputAction :type Input%20Action%20Object%20Reference :default "/Game/Controls/IA_MoveAmy.IA_MoveAmy"))
  (bind _returnvalue (Pawn|GetControlRotation :!class /Script/Engine.Pawn))
  (bind _returnvalue_2 (Math|Rotator|MakeRotator 0.0 0.0 (.yaw _returnvalue)))
  (Pawn|Input|AddMovementInput (Math|Vector|GetForwardVector _returnvalue_2) (.x ActionValue) false)
  (Pawn|Input|AddMovementInput (Math|Vector|GetRightVector _returnvalue_2) (.y ActionValue) false))

(event Input|EnhancedActionEvents|EnhancedInputActionIA_JumpAmy
  (params (ActionValue :type Boolean) (ElapsedSeconds :type Float%20%28double-precision%29) (TriggeredSeconds :type Float%20%28double-precision%29) (InputAction :type Input%20Action%20Object%20Reference :default "/Game/Controls/IA_JumpAmy.IA_JumpAmy"))
  (Character|Jump))

(event EventBeginPlay)

(event Collision|EventActorBeginOverlap
  (params (OtherActor :type Actor%20Object%20Reference)))

(event EventTick
  (params (DeltaSeconds :type Float%20%28single-precision%29))
  (Variables|Default|Setspeed (Math|Vector|VectorLengthXY (Transformation|GetVelocity))))

(event Input|MouseEvents|LeftMouseButton
  (params (Key :type Key%20Structure :default "None"))
  (bind _mesh (Variables|Character|GetMesh))
  (:Pressed
    (if (not (Variables|Default|GetWaving?))
      (Utilities|FlowControl|DoOnce false :!label _label
        (:Completed
          (Animation|Montage|PlayMontage _mesh "/Game/Animtaions/ComboAction.ComboAction" 1.0 0.0 "LPunch"
            (:OnBlendOut
              (Animation|Montage|PlayMontage _mesh "/Game/Animtaions/ComboAction.ComboAction" 1.0 0.0 "RPunch"
                (:OnBlendOut
                  (goto _label Reset))
                (:OnInterrupted
                  (goto _label Reset))))
            (:OnInterrupted
              (goto _label Reset))))))))

(event Input|KeyboardEvents|H
  (params (Key :type Key%20Structure :default "None"))
  (:Pressed
    (Variables|Default|SetWaving? true)
    (Animation|Montage|PlayMontage (Variables|Character|GetMesh) "/Game/Animtaions/ComboAction.ComboAction" 1.0 0.0 "Waving"))
  (:Released
    (Variables|Default|SetWaving? false)
    (Animation|StopAnimMontage 0)))

(fn ConstructionScript)